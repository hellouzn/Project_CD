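; BP_Monster is a monster spawner that creates a random monster at its own transform.
; BeginPlay starts a looping timer that calls SpawnMonster every two seconds.
; SpawnMonster favors BP_Monster1 through a weighted random roll, then rolls again to choose between the others, making BP_Monster3 uncommon and BP_Monster2 rarest.
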(event EventBeginPlay
  (Utilities|Time|SetTimerbyFunctionName 0 "spawnMonster" 2.0 true))

(event Collision|EventActorBeginOverlap
  (params (OtherActor :type Actor%20Object%20Reference)))

(event EventTick
  (params (DeltaSeconds :type Float%20%28single-precision%29)))

(fn ConstructionScript)

(fn SpawnMonster
  (bind _returnvalue (Math|Random|RandomInteger 9))
  (if (<= _returnvalue 7)
    (Game|SpawnActorfromClass "/Game/BP/BP_Monster1.BP_Monster1_C" (Transformation|GetActorTransform) "Undefined" "MultiplyWithRoot" 0 0)
    (elif (== _returnvalue 8)
      (Game|SpawnActorfromClass "/Game/BP/BP_Monster2.BP_Monster2_C" (Transformation|GetActorTransform) "Undefined" "MultiplyWithRoot" 0 0)
      (else
        (Game|SpawnActorfromClass "/Game/BP/BP_Monster3.BP_Monster3_C" (Transformation|GetActorTransform) "Undefined" "MultiplyWithRoot" 0 0)))))